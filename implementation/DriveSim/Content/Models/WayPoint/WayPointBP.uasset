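; Waypoint actor that shows the player's distance to it on an icon widget.
; On BeginPlay it caches the IconWidget from its widget component.
; Each Tick, the widget computes the distance between the player pawn and the waypoint, and the truncated integer value is passed back to the widget's Update.
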(event `self.ReceiveBeginPlay`
  (bind _asicon_widget (cast `/Game/Models/WayPoint/IconWidget` (`WidgetComponent.GetUserWidgetObject` (`self.Icon_Widget`))))
  (set `self.IconWRef` _asicon_widget))

(event `self.ReceiveTick`
  (params (DeltaSeconds :type "Float (single-precision)"))
  (bind _iconwref (`self.IconWRef`))
  (bind _returnvalue (`/Game/Models/WayPoint/IconWidget.GetDistance` _iconwref (`GameplayStatics.GetPlayerPawn` 0) self))
  (`/Game/Models/WayPoint/IconWidget.Update` _iconwref (`KismetMathLibrary.FTrunc` _returnvalue)))

(fn `UserConstructionScript`)