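; PedestrianSpawnPoint is a spawn point actor that keeps one AI unit of a configurable class in the world.
; BeginPlay spawns the unit at the actor's location through SpawnAIFromClass and stores it in SpawnedUnit.
; Tick polls that reference and, when it is no longer valid, waits RespawnTimer through a Delay before calling Respawn to spawn a replacement.
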(event `Respawn`
  (bind _returnvalue (`AIBlueprintHelperLibrary.SpawnAIFromClass` (`self.ClassToSpawn`) null (`self.K2_GetActorLocation`) :!label _label))
  (set `self.SpawnedUnit` _returnvalue))

(event `self.ReceiveBeginPlay`
  (goto _label))

(event `self.ReceiveTick`
  (params (DeltaSeconds :type "Float (single-precision)"))
  (if (not (`KismetSystemLibrary.IsValid` (`self.SpawnedUnit`)))
    (`KismetSystemLibrary.Delay` (`self.RespawnTimer`))
    (`self.Respawn`)))

(fn `UserConstructionScript`)