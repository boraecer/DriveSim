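; VehicleAI is an AI traffic vehicle that drives toward a target through its VehicleAIController, starting 15 seconds after BeginPlay.
; Hit-box overlaps with other VehicleAI or the player's Sedan stop movement immediately, then resume the last target when the overlap ends.
; IsPlayerBox checks XY proximity between a supplied box location and its own Box, then respawns the vehicle, restarts its route and deducts Sedan points.
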(event `Set Player Location`
  (params (`Player Location` :type "Vector Structure"))
  ;[1 1 1] Set Player Sedan Location for overlapping with VehicleAI
  (set `self.PlayerLocationVector` `Player Location`))

(event `self.ReceiveBeginPlay`
  ;[1 1 1] Vehicle AI Spawn Point Set
  (set `self.SpawnPoint` (`self.K2_GetActorLocation` self))
  ;[1 1 1] Vehicle AI Loop
  (`KismetSystemLibrary.Delay` 15.0)
  (`self.SetNextTarget` (`self.AI Target`)))

(event `IsPlayerBox`
  (params (OverlappedBox :type "Vector Structure"))
  (bind (_returnvalue_x _returnvalue_y) (`KismetMathLibrary.BreakVector` (`SceneComponent.K2_GetComponentLocation` (`self.Box`))))
  ;[1 1 1] Vehicle AI Overlap With Player Sedan (New Version)
  (if (<= (`KismetMathLibrary.VSizeXY` (- (`KismetMathLibrary.MakeVector` OverlappedBox_X OverlappedBox_Y) (`KismetMathLibrary.MakeVector` _returnvalue_x _returnvalue_y))) 50.0)
    (`self.K2_SetActorTransform` self (`KismetMathLibrary.MakeTransform` (`self.SpawnPoint`)) false false)
    (`self.SetNextTarget` (`self.AI Target`))
    (bind _assedan (cast `/Game/VehicleBP/Sedan/Sedan` (`GameplayStatics.GetPlayerPawn` 0)))
    (set `/Game/VehicleBP/Sedan/Sedan.points` (- (`/Game/VehicleBP/Sedan/Sedan.points` _assedan) 10) _assedan)))

(event `self.VehicleHitBox.OnComponentBeginOverlap`
  (params (OverlappedComponent :type "PrimitiveComponent Object Reference") (OtherActor :type "Actor Object Reference") (OtherComp :type "PrimitiveComponent Object Reference") (OtherBodyIndex :type Integer) (bFromSweep :type Boolean) (SweepResult :type "HitResult Structure (by ref)"))
  (cast `/Game/Blueprints/VehicleAI` OtherActor)
  (`self.StopMoving` self))

(event `self.VehicleHitBox.OnComponentEndOverlap`
  (params (OverlappedComponent :type "PrimitiveComponent Object Reference") (OtherActor :type "Actor Object Reference") (OtherComp :type "PrimitiveComponent Object Reference") (OtherBodyIndex :type Integer))
  (cast `/Game/Blueprints/VehicleAI` OtherActor)
  (`self.SetNextTarget` (`self.OnGoingTarget`)))

(event `self.SedanHitBox.OnComponentBeginOverlap`
  (params (OverlappedComponent :type "PrimitiveComponent Object Reference") (OtherActor :type "Actor Object Reference") (OtherComp :type "PrimitiveComponent Object Reference") (OtherBodyIndex :type Integer) (bFromSweep :type Boolean) (SweepResult :type "HitResult Structure (by ref)"))
  (cast `/Game/VehicleBP/Sedan/Sedan` OtherActor)
  (`self.StopMoving`))

(event `self.SedanHitBox.OnComponentEndOverlap`
  (params (OverlappedComponent :type "PrimitiveComponent Object Reference") (OtherActor :type "Actor Object Reference") (OtherComp :type "PrimitiveComponent Object Reference") (OtherBodyIndex :type Integer))
  (cast `/Game/VehicleBP/Sedan/Sedan` OtherActor)
  (`self.SetNextTarget` (`self.OnGoingTarget`)))

(fn `SetNextTarget`
  (params (`Next Target` :type "Character Object Reference"))
  (locals (CurrentTarget :type "Character Object Reference"))
  (bind _output_get (set `local.CurrentTarget` `Next Target`))
  (bind _asvehicle_aicontroller (cast `/Game/Blueprints/VehicleAIController` (`AIBlueprintHelperLibrary.GetAIController` self)))
  (`/Game/Blueprints/VehicleAIController.MoveToTarget` _asvehicle_aicontroller _output_get)
  (set `self.OnGoingTarget` _output_get))

(fn `StopMoving`
  (bind _asvehicle_ai (cast `/Game/Blueprints/VehicleAI` self))
  (`MovementComponent.StopMovementImmediately` (`Character.CharacterMovement` _asvehicle_ai)))

(fn `UserConstructionScript`)